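; BP_Camera is a camera actor built to turn toward a BP_BodyChar near its ThreatSphere and otherwise ease back to its starting rotation.
; Tick interpolates the Rotator component's world rotation toward the cached character when GuyInRange is true, or more slowly toward the actor rotation saved at BeginPlay.
; Begin overlap caches the character, but both overlap events set GuyInRange false, so this graph never activates tracking.
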(event OnComponentBeginOverlap(ThreatSphere)
  (params (OverlappedComponent :type Primitive%20Component%20Object%20Reference) (OtherActor :type Actor%20Object%20Reference) (OtherComp :type Primitive%20Component%20Object%20Reference) (OtherBodyIndex :type Integer) (bFromSweep :type Boolean) (SweepResult :type Hit%20Result%20Structure%20%28by%20ref%29))
  (bind _asbp_body_char (Utilities|Casting|CastToBP_BodyChar OtherActor))
  (Variables|Default|SetGuyInRange? false))

(event OnComponentEndOverlap(ThreatSphere)
  (params (OverlappedComponent :type Primitive%20Component%20Object%20Reference) (OtherActor :type Actor%20Object%20Reference) (OtherComp :type Primitive%20Component%20Object%20Reference) (OtherBodyIndex :type Integer))
  (Utilities|Casting|CastToBP_BodyChar OtherActor)
  (Variables|Default|SetGuyInRange? false))

(event EventTick
  (params (DeltaSeconds :type Float%20%28single-precision%29))
  (bind _rotator (Variables|Default|GetRotator))
  (bind _returnvalue (Transformation|GetWorldRotation _rotator))
  (if (Variables|Default|GetGuyInRange?)
    (Transformation|SetWorldRotation _rotator (Math|Interpolation|RInterpTo _returnvalue (Math|Rotator|FindLookatRotation (Transformation|GetWorldLocation _rotator) (Transformation|GetActorLocation (stale OnComponentBeginOverlap(ThreatSphere) _asbp_body_char))) DeltaSeconds 2.0) false false)
    (else
      (Transformation|SetWorldRotation _rotator (Math|Interpolation|RInterpTo _returnvalue (Variables|Default|GetDefaultRotation) DeltaSeconds 1.0) false false))))

(event EventBeginPlay
  (Variables|Default|SetDefaultRotation (Transformation|GetActorRotation)))

(fn ConstructionScript)